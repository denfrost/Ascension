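; AttackMotion is an anim notify state that drives attack movement on the owning actor's AttackComponent during an animation window.
; Notify begin calls SetupMotion and notify end calls FinishMotion on that component.
; Each tick reads the MotionX, MotionY and MotionZ animation curves from the anim instance and passes them as a vector to AttackMotion, so movement is authored as curves in the animation.
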(fn `Received_NotifyBegin`
  (params (MeshComp :type "SkeletalMeshComponent Object Reference") (Animation :type "AnimSequenceBase Object Reference") (TotalDuration :type "Float (double-precision)"))
  (returns (ReturnValue :type Boolean))
  (bind _returnvalue (`Actor.GetComponentByClass` (`ActorComponent.GetOwner` MeshComp) "/Script/Ascension.AttackComponent"))
  (`/Engine/EditorBlueprintResources/StandardMacros.IsValid` _returnvalue
    (:`Is Valid`
      (`AttackComponent.SetupMotion` _returnvalue)
      (return true))
    (:`Is Not Valid`
      (return false))))

(fn `Received_NotifyEnd`
  (params (MeshComp :type "SkeletalMeshComponent Object Reference") (Animation :type "AnimSequenceBase Object Reference"))
  (returns (ReturnValue :type Boolean))
  (bind _returnvalue (`Actor.GetComponentByClass` (`ActorComponent.GetOwner` MeshComp) "/Script/Ascension.AttackComponent"))
  (`/Engine/EditorBlueprintResources/StandardMacros.IsValid` _returnvalue
    (:`Is Valid`
      (`AttackComponent.FinishMotion` _returnvalue)
      (return true))
    (:`Is Not Valid`
      (return false))))

(fn `Received_NotifyTick`
  (params (MeshComp :type "SkeletalMeshComponent Object Reference") (Animation :type "AnimSequenceBase Object Reference") (FrameDeltaTime :type "Float (double-precision)"))
  (returns (ReturnValue :type Boolean))
  (bind _returnvalue (`SkeletalMeshComponent.GetAnimInstance` MeshComp))
  (bind _returnvalue_2 (`Actor.GetComponentByClass` (`ActorComponent.GetOwner` MeshComp) "/Script/Ascension.AttackComponent"))
  (`/Engine/EditorBlueprintResources/StandardMacros.IsValid` _returnvalue_2
    (:`Is Valid`
      (`AttackComponent.AttackMotion` _returnvalue_2 (`KismetMathLibrary.MakeVector` (`AnimInstance.GetCurveValue` _returnvalue "MotionX") (`AnimInstance.GetCurveValue` _returnvalue "MotionY") (`AnimInstance.GetCurveValue` _returnvalue "MotionZ")))
      (return true))
    (:`Is Not Valid`
      (return false))))