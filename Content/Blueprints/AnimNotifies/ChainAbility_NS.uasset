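; ChainAbility_NS is an anim notify state that marks a window in an animation for chaining player abilities.
; On begin and end it calls SetCanChain on the owner's PlayerAbilitySystemComponent, passing CanChain both times.
; Each tick it finds the PlayerInputComponent on the owning Character's controller and calls TryBufferedAction, so buffered input can fire during the window.
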(fn `Received_NotifyBegin`
  (params (MeshComp :type "SkeletalMeshComponent Object Reference") (Animation :type "AnimSequenceBase Object Reference") (TotalDuration :type "Float (double-precision)"))
  (returns (ReturnValue :type Boolean))
  (locals (CanChain :type Boolean :default true))
  (bind _returnvalue (`Actor.GetComponentByClass` (`ActorComponent.GetOwner` MeshComp) "/Script/Ascension.PlayerAbilitySystemComponent"))
  (`/Engine/EditorBlueprintResources/StandardMacros.IsValid` _returnvalue
    (:`Is Valid`
      (`PlayerAbilitySystemComponent.SetCanChain` _returnvalue (`local.CanChain`))
      (return true))
    (:`Is Not Valid`
      (return false))))

(fn `Received_NotifyEnd`
  (params (MeshComp :type "SkeletalMeshComponent Object Reference") (Animation :type "AnimSequenceBase Object Reference"))
  (returns (ReturnValue :type Boolean))
  (locals (CanChain :type Boolean))
  (bind _returnvalue (`Actor.GetComponentByClass` (`ActorComponent.GetOwner` MeshComp) "/Script/Ascension.PlayerAbilitySystemComponent"))
  (`/Engine/EditorBlueprintResources/StandardMacros.IsValid` _returnvalue
    (:`Is Valid`
      (`PlayerAbilitySystemComponent.SetCanChain` _returnvalue (`local.CanChain`))
      (return true))
    (:`Is Not Valid`
      (return false))))

(fn `Received_NotifyTick`
  (params (MeshComp :type "SkeletalMeshComponent Object Reference") (Animation :type "AnimSequenceBase Object Reference") (FrameDeltaTime :type "Float (double-precision)"))
  (returns (ReturnValue :type Boolean))
  (bind _ascharacter (cast `Character` (`ActorComponent.GetOwner` MeshComp))
    (:`then`
      (bind _returnvalue (`Pawn.GetController` _ascharacter))
      (`/Engine/EditorBlueprintResources/StandardMacros.IsValid` _returnvalue
        (:`Is Valid`
          (bind _returnvalue_2 (`Actor.GetComponentByClass` _returnvalue "/Script/Ascension.PlayerInputComponent"))
          (`/Engine/EditorBlueprintResources/StandardMacros.IsValid` _returnvalue_2
            (:`Is Valid`
              (`PlayerInputComponent.TryBufferedAction` _returnvalue_2)
              (return true))
            (:`Is Not Valid`
              _)))
        (:`Is Not Valid`
          _)))
    (:`CastFailed`
      _))
  (return false))