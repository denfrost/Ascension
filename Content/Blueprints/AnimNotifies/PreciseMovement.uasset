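; Anim notify state that drives curve-authored movement on the owning actor during its window in an animation.
; Each tick it reads the MotionX, MotionY and MotionZ curves from the mesh's anim instance and scales them by MaxVelocity.
; The resulting velocity goes to PerformMove on the owner's GameMovementComponent with the frame delta time; the tick returns false when that component is missing.
; Begin and end events do nothing beyond returning true.
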(fn `Received_NotifyBegin`
  (params (MeshComp :type "SkeletalMeshComponent Object Reference") (Animation :type "AnimSequenceBase Object Reference") (TotalDuration :type "Float (double-precision)"))
  (returns (ReturnValue :type Boolean))
  (return true))

(fn `Received_NotifyEnd`
  (params (MeshComp :type "SkeletalMeshComponent Object Reference") (Animation :type "AnimSequenceBase Object Reference"))
  (returns (ReturnValue :type Boolean))
  (return true))

(fn `Received_NotifyTick`
  (params (MeshComp :type "SkeletalMeshComponent Object Reference") (Animation :type "AnimSequenceBase Object Reference") (FrameDeltaTime :type "Float (double-precision)"))
  (returns (ReturnValue :type Boolean))
  (bind _returnvalue (`SkeletalMeshComponent.GetAnimInstance` MeshComp))
  (bind _maxvelocity (`self.MaxVelocity`))
  (bind _returnvalue_2 (`Actor.GetComponentByClass` (`ActorComponent.GetOwner` MeshComp) "/Script/Ascension.GameMovementComponent"))
  (`/Engine/EditorBlueprintResources/StandardMacros.IsValid` _returnvalue_2
    (:`Is Valid`
      (`GameMovementComponent.PerformMove` _returnvalue_2 (`KismetMathLibrary.MakeVector` (* (`AnimInstance.GetCurveValue` _returnvalue "MotionX") _maxvelocity) (* (`AnimInstance.GetCurveValue` _returnvalue "MotionY") _maxvelocity) (* (`AnimInstance.GetCurveValue` _returnvalue "MotionZ") _maxvelocity)) FrameDeltaTime)
      (return true))
    (:`Is Not Valid`
      (return false))))