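; Goblin melee enemy that enters combat when AI perception senses a player-tagged actor and exits when a stimulus is lost.
; The construction script gives its attack component the sword hitbox and three slash montage attacks with knockback, while events forward damage-window and completion calls to it.
; Taking a hit shows effects, interrupts any attack, then plays an impact montage or kills and later destroys the goblin.
; A widget health bar can be shown or hidden.
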(event `self.ApplyHitEffect`
  (params (SourceActor :type "Actor Object Reference") (Damage :type "Float (single-precision)") (HitEffect :type "EHitEffect Enum" :default "HE_PushBack") (AttackEffect :type "AttackEffect Structure"))
  ;[1 1 1] Interface Overrides
  ;;[1 1 1] Applying Attack Effects
  (if (not (`self.Dead`))
    (`self.ShowHitVisuals`)
    (`self.ApplyAttackEffects` SourceActor Damage HitEffect AttackEffect)
    (if (`|EnumEquality` (`self.ActionState`) "ES_Attacking")
      (`self.ResetAttack`)
      (`AttackComponent.OnAttackComplete` (`self.GoblinAttackComponent`) false))
    (bind _returnvalue (`self.CheckDead`))
    (if _returnvalue
      (`self.KillActor`)
      (`KismetSystemLibrary.Delay` 5.0)
      (`self.K2_DestroyActor`)
      (else
        (`self.PlayAnimMontage` "/Game/Blueprints/Enemies/Goblin/AnimMontages/GS_Impact.GS_Impact" 1.5)
        (`self.OnHit`)))))

(event `self.ShowHitVisuals`
  ;[1 1 1] Blueprint Overrides
  ;;[1 1 1] Show Hit Visuals
  (bind _returnvalue (`GameplayStatics.SpawnEmitterAtLocation` "/Game/Assets/StarterContent/Particles/P_HitEffect.P_HitEffect" (`SceneComponent.K2_GetComponentLocation` (`self.HitEffectLocation`))))
  (`SceneComponent.SetRelativeScale3D` _returnvalue (0.7 0.7 0.7))
  (`GameplayStatics.PlaySoundAtLocation` "/Game/Assets/Audio/HitEffectCue.HitEffectCue" (`SceneComponent.K2_GetComponentLocation` (`self.HitEffectLocation`))))

(event `self.ReceiveBeginPlay`
  ;[1 1 1] Setup Health Bar
  (bind _ashealth_bar (cast `/Game/Blueprints/Widgets/HealthBar` (`WidgetComponent.GetUserWidgetObject` (`self.HealthBar`))))
  (set `/Game/Blueprints/Widgets/HealthBar.OwningActor` self _ashealth_bar))

(event `self.KillActor`
  ;[1 1 1] Blueprint Overrides
  ;;[1 1 1] Kill Actor
  (`parent.KillActor`)
  (`self.PlayAnimMontage` "/Game/Blueprints/Enemies/Goblin/AnimMontages/fallback_death.fallback_death")
  (`PrimitiveComponent.SetCollisionEnabled` (`self.CapsuleComponent`) "NoCollision"))

(event `self.ShowHealthBar`
  ;[1 1 1] Interface Overrides
  ;;[1 1 1] Show/Hide Health Bar
  (`SceneComponent.SetHiddenInGame` (`self.HealthBar`) false false))

(event `self.AttackComplete`
  ;[1 1 1] Attack Complete Broadcast
  (`AttackComponent.OnAttackComplete` (`self.GoblinAttackComponent`) true))

(event `self.HideHealthBar`
  ;[1 1 1] Interface Overrides
  ;;[1 1 1] Show/Hide Health Bar
  (`SceneComponent.SetHiddenInGame` (`self.HealthBar`) true false))

(event `self.AIPerception.OnTargetPerceptionUpdated`
  (params (Actor :type "Actor Object Reference") (Stimulus :type "AIStimulus Structure"))
  ;[1 1 1] AI Perception
  (bind _returnvalue (`self.IsDead`))
  (if _returnvalue
    _
    (elif (`.bSuccessfullySensed` (break `AIStimulus` Stimulus))
      (if (`self.ActorHasTag` Actor "Player")
        (`self.EnterCombat` Actor))
      (else
        (`self.ExitCombat`)))))

(event `Slash Sound`
  ;[1 1 1] Audio
  ;;[1 1 1] Sword Slash Sound
  (`GameplayStatics.PlaySoundAtLocation` "/Game/Assets/Audio/SlashCue.SlashCue" (`SceneComponent.K2_GetComponentLocation` (`self.SlashLoc`))))

(event `self.FootstepSound`
  ;[1 1 1] Audio
  ;;[1 1 1] Footsounds (TODO: Implement This)
)

(event `DisableDamage`
  ;[1 1 1] Attack Functionality
  (`AttackComponent.DisableDamage` (`self.GoblinAttackComponent`)))

(event `EnableDamage`
  ;[1 1 1] Attack Functionality
  (`AttackComponent.EnableDamage` (`self.GoblinAttackComponent`)))

(event `ClearDamagedActors`
  ;[1 1 1] Attack Functionality
  (`AttackComponent.ClearDamagedActors` (`self.GoblinAttackComponent`)))

(fn `UserConstructionScript`
  (bind _goblinattackcomponent (`self.GoblinAttackComponent`))
  (set `self.AttackComponent` _goblinattackcomponent)
  (set `AttackComponent.AttackHitBox` (`self.SwordHitBox`) _goblinattackcomponent)
  ;[1 1 1] Creating Goblin Attacks
  (`AttackComponent.CreateAttack` _goblinattackcomponent "Attack01" (make `Attack` "/Game/Blueprints/Enemies/Goblin/AnimMontages/gs_slash_1.gs_slash_1" 0.0 2048.0 null "HE_PushBack" 10.0 (make `AttackEffect` 5000.0)))
  (`AttackComponent.CreateAttack` _goblinattackcomponent "Attack02" (make `Attack` "/Game/Blueprints/Enemies/Goblin/AnimMontages/gs_slash_2.gs_slash_2" 0.0 2048.0 null "HE_PushBack" 10.0 (make `AttackEffect` 5000.0)))
  (`AttackComponent.CreateAttack` _goblinattackcomponent "Attack03" (make `Attack` "/Game/Blueprints/Enemies/Goblin/AnimMontages/gs_slash_3.gs_slash_3" 0.0 2048.0 null "HE_PushBack" 10.0 (make `AttackEffect` 5000.0))))