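; AI controller for the Goblin enemy that starts its behavior tree and tracks a perceived player.
; On BeginPlay it loads the PatrolData blackboard, resets the index key to zero and runs Goblin_BT.
; AI Perception updates store a sensed Player-tagged actor in the enemy key.
; Any unsuccessful sense update clears that key, whatever the actor, with debug prints for found and lost.
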(event `self.ReceiveBeginPlay`
  (bind _blackboardcomponent (`self.UseBlackboard` "/Game/Blueprints/Enemies/Goblin/AI/PatrolData.PatrolData"))
  (set `self.BlackboardComp` _blackboardcomponent)
  (`BlackboardComponent.SetValueAsInt` _blackboardcomponent (`self.IndexKeyName`) 0)
  (`self.RunBehaviorTree` "/Game/Blueprints/Enemies/Goblin/AI/Goblin_BT.Goblin_BT"))

(event `self.AIPerception.OnTargetPerceptionUpdated`
  (params (Actor :type "Actor Object Reference") (Stimulus :type "AIStimulus Structure"))
  (bind _blackboardcomp (`self.BlackboardComp`))
  (bind _enemykeyname (`self.EnemyKeyName`))
  (if (`.bSuccessfullySensed` (break `AIStimulus` Stimulus))
    (if (`self.ActorHasTag` Actor "Player")
      (`BlackboardComponent.SetValueAsObject` _blackboardcomp _enemykeyname Actor)
      (`KismetSystemLibrary.PrintString` "Found"))
    (else
      (`BlackboardComponent.ClearValue` _blackboardcomp _enemykeyname)
      (`KismetSystemLibrary.PrintString` "Not Found"))))

(fn `UserConstructionScript`)