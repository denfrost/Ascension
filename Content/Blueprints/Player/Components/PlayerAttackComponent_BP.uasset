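; Player attack component that picks which combo attack to perform for a light or strong attack request.
; SelectAttack branches on the attack type string, then switches on ComboMeter to look up the first, second or third attack in that chain by name via GetAttack and pass it to SetAttack.
; Both types share one ComboMeter, which advances each call and resets to one, replaying the opener, when out of range.
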(event `self.SelectAttack`
  (params (AttackType :type String))
  (bind _combometer (`self.ComboMeter`))
  (bind _returnvalue (+ _combometer 1))
  ;[1 1 1] Selecting Attack To Perform
  (if (`KismetStringLibrary.EqualEqual_StrStr` AttackType "Light Attack")
    ;;[1 1 1] Light Attacks
    (switch `int` _combometer
      (:`Default`
        (set `self.ComboMeter` 1)
        (bind (_found _attack) (`self.GetAttack` "Light01"))
        (`self.SetAttack` _found _attack))
      (:`0`
        (set `self.ComboMeter` _returnvalue)
        (bind (_found_2 _attack_2) (`self.GetAttack` "Light01"))
        (`self.SetAttack` _found_2 _attack_2))
      (:`1`
        (set `self.ComboMeter` _returnvalue)
        (bind (_found_3 _attack_3) (`self.GetAttack` "Light02"))
        (`self.SetAttack` _found_3 _attack_3))
      (:`2`
        (set `self.ComboMeter` _returnvalue)
        (bind (_found_4 _attack_4) (`self.GetAttack` "Light03"))
        (`self.SetAttack` _found_4 _attack_4)))
    (elif (`KismetStringLibrary.EqualEqual_StrStr` AttackType "Strong Attack")
      ;;[1 1 1] Strong Attacks
      (switch `int` _combometer
        (:`Default`
          (set `self.ComboMeter` 1)
          (bind (_found_5 _attack_5) (`self.GetAttack` "Strong01"))
          (`self.SetAttack` _found_5 _attack_5))
        (:`0`
          (set `self.ComboMeter` _returnvalue)
          (bind (_found_6 _attack_6) (`self.GetAttack` "Strong01"))
          (`self.SetAttack` _found_6 _attack_6))
        (:`1`
          (set `self.ComboMeter` _returnvalue)
          (bind (_found_7 _attack_7) (`self.GetAttack` "Strong02"))
          (`self.SetAttack` _found_7 _attack_7))
        (:`2`
          (set `self.ComboMeter` _returnvalue)
          (bind (_found_8 _attack_8) (`self.GetAttack` "Strong03"))
          (`self.SetAttack` _found_8 _attack_8))))))