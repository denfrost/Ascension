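; Player character Blueprint for sword-and-shield melee combat with camera lock-on.
; Construction binds the sword hitbox to AttackComponent and registers light, strong and dodge abilities with AbilitySystemComponent.
; LockOn targets a living Lockable pawn in EnemyDetectRadius, which also toggles enemy health bars; Tick turns the camera toward it until dead or out of range.
; Events handle sword trails, sheathing, sounds and hit reactions; an experimental flying attack is left unconnected.
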(event `TrailStart`
  ;[1 1 1] AnimTrail for the sword
  (`ParticleSystemComponent.BeginTrails` (`self.SwordTrail`) "TrailStart" "TrailEnd" "ETrailWidthMode_FromCentre" 2.0))

(event `self.ReceiveTick`
  (params (DeltaSeconds :type "Float (single-precision)"))
  (bind _lockedactor (`self.LockedActor`))
  ;[1 1 1] Camera Lock On  |  TODO: Refactor this into C++
  (if (and (`self.LockedOn`) (`KismetSystemLibrary.IsValid` _lockedactor))
    (if (>= (`self.GetDistanceTo` self _lockedactor) (`SphereComponent.SphereRadius` (`self.EnemyDetectRadius`)))
      (`self.LockOff` :!label _label)
      (else
        ;;[1 1 1] Check If Target Is Dead
        (if (`KismetSystemLibrary.DoesImplementInterface` _lockedactor "/Script/Ascension.Damageable")
          (bind _returnvalue (message `Damageable.IsDead` _lockedactor))
          (if _returnvalue
            (goto _label)
            (else
              _)))
        ;;[1 1 1] Lock Camera Onto The Target
        (`Controller.SetControlRotation` (`self.GetController`) (`KismetMathLibrary.RInterpTo` (`self.GetControlRotation`) (`KismetMathLibrary.MakeRotator` 0.0 -5.0 (.yaw (`KismetMathLibrary.FindLookAtRotation` (`SceneComponent.K2_GetComponentLocation` (`self.FollowCamera`)) (`self.K2_GetActorLocation` _lockedactor)))) DeltaSeconds 5.0))))))

(event `self.SlashSound`
  ;[1 1 1] Audio
  ;;[1 1 1] Slash Sounds
  (`GameplayStatics.PlaySoundAtLocation` "/Game/Assets/Audio/SlashCue.SlashCue" (`SceneComponent.K2_GetComponentLocation` (`self.SlashLoc`)) (struct) 1.0 1.0 0.0 null null null))

(event `TrailEnd`
  ;[1 1 1] AnimTrail for the sword
  (`ParticleSystemComponent.EndTrails` (`self.SwordTrail`)))

(event `self.FootstepSound`
  ;[1 1 1] Audio
  ;;[1 1 1] Footsteps
  (if (`|EnumEquality` (`PlayerStateComponent.GetCharacterState` (`self.StateComponent`)) "CS_Idle")
    (`/Engine/EditorBlueprintResources/StandardMacros.FlipFlop`
      (:`A`
        (`GameplayStatics.PlaySoundAtLocation` "/Game/Assets/Audio/FootstepCue.FootstepCue" (`SceneComponent.K2_GetComponentLocation` (`self.LFoot`)) (struct) 1.0 1.0 0.0 null null null))
      (:`B`
        (`GameplayStatics.PlaySoundAtLocation` "/Game/Assets/Audio/FootstepCue.FootstepCue" (`SceneComponent.K2_GetComponentLocation` (`self.RFoot`)) (struct) 1.0 1.0 0.0 null null null)))))

(event `self.Unsheathed`
  ;[1 1 1] Sheathing/Unsheathing
  (`SceneComponent.SetHiddenInGame` (`self.Sword`) false false)
  (`SceneComponent.SetHiddenInGame` (`self.Shield`) false false)
  (`SceneComponent.SetHiddenInGame` (`self.SheathedShield`) true false)
  (`SceneComponent.SetHiddenInGame` (`self.SheathedSword`) true false))

(event `self.Impact`
  (params (Direction :type "Vector Structure (by ref)"))
  ;[1 1 1] Player Receiving Damage
  (`parent.Impact` Direction)
  (`self.PlayAnimMontage` "/Game/Blueprints/Player/AnimMontages/Impact01.Impact01")
  (`GameplayStatics.PlaySoundAtLocation` "/Game/Assets/Audio/HitEffectCue.HitEffectCue" (`SceneComponent.K2_GetComponentLocation` (`self.HitLocation`)) (struct) 1.0 1.0 0.0 null null null))

(event `self.Sheathed`
  ;[1 1 1] Sheathing/Unsheathing
  (`SceneComponent.SetHiddenInGame` (`self.SheathedShield`) false false)
  (`SceneComponent.SetHiddenInGame` (`self.SheathedSword`) false false)
  (`SceneComponent.SetHiddenInGame` (`self.Sword`) true false)
  (`SceneComponent.SetHiddenInGame` (`self.Shield`) true false))

(event `InputAction|LockOn`
  (params (Key :type "Key Structure"))
  ;[1 1 1] Camera Lock On  |  TODO: Refactor this into C++
  ;;[1 1 1] Lock On Input
  (:`Pressed`
    (if (`self.LockedOn`)
      (`self.LockOff`)
      (else
        (`self.LockOn`)))))

(event `self.EnemyDetectRadius.OnComponentBeginOverlap`
  (params (OverlappedComponent :type "PrimitiveComponent Object Reference") (OtherActor :type "Actor Object Reference") (OtherComp :type "PrimitiveComponent Object Reference") (OtherBodyIndex :type Integer) (bFromSweep :type Boolean) (SweepResult :type "HitResult Structure (by ref)"))
  ;[1 1 1] Displaying Enemy Health Bars
  (if (`KismetSystemLibrary.DoesImplementInterface` OtherActor "/Script/Ascension.Damageable")
    (message `Damageable.ShowHealthBar` OtherActor)))

(event `self.EnemyDetectRadius.OnComponentEndOverlap`
  (params (OverlappedComponent :type "PrimitiveComponent Object Reference") (OtherActor :type "Actor Object Reference") (OtherComp :type "PrimitiveComponent Object Reference") (OtherBodyIndex :type Integer))
  ;[1 1 1] Displaying Enemy Health Bars
  (if (`KismetSystemLibrary.DoesImplementInterface` OtherActor "/Script/Ascension.Damageable")
    (message `Damageable.HideHealthBar` OtherActor)))

(event `Key|K`
  (params (Key :type "Key Structure"))
  ;[1 0.01404 0] EXPERIMENTAL: 3D Attacks
)

(fn `AddAbility`
  (params (AbilityName :type String) (Class :type "Ability Class Reference"))
  (`GameAbilitySystemComponent.AddAbility` (`self.AbilitySystemComponent`) AbilityName Class))

(fn `CharacterImpact`)

(fn `GetHealthPercent`
  (returns (HealthPercent :type "Float (double-precision)"))
  (return (`self.GetHealthPercentage`)))

(fn `IsDead`
  (returns (ReturnValue :type Boolean))
  (return false))

(fn `LockOff`
  (set `self.LockedActor` null)
  (set `self.LockedOn` false))

(fn `LockOn`
  (locals (MinDistance :type "Float (double-precision)" :default 1000000.0))
  (for _array_element (`PrimitiveComponent.GetOverlappingActors` (`self.EnemyDetectRadius`) "/Script/Engine.Pawn")
    (if (and (`KismetSystemLibrary.DoesImplementInterface` _array_element "/Script/Ascension.Lockable") (!= _array_element self))
      (if (`KismetSystemLibrary.DoesImplementInterface` _array_element "/Script/Ascension.Damageable")
        (bind _returnvalue (message `Damageable.IsDead` _array_element))
        (if (not _returnvalue)
          (if (<= (`self.GetDistanceTo` _array_element null) (`local.MinDistance`)) :!label _label
            (set `self.LockedActor` _array_element)
            (set `self.LockedOn` true)))
        (else
          (goto _label))))))

(fn `UserConstructionScript`
  (set `AttackComponent.AttackHitBox` (`self.SwordHitBox`) (`self.AttackComponent`))
  (`GameAbilitySystemComponent.ClearAbilities` (`self.AbilitySystemComponent`))
  ;[1 1 1] Move this to C++/Refactor
  (`|ExecutionSequence`
    (:`then_0`
      (`self.AddAbility` "Light01" "/Game/Blueprints/Player/Abilities/Attacks/Light01.Light01_C"))
    (:`then_1`
      (`self.AddAbility` "Light02" "/Game/Blueprints/Player/Abilities/Attacks/Light02.Light02_C"))
    (:`then_2`
      (`self.AddAbility` "Light03" "/Game/Blueprints/Player/Abilities/Attacks/Light03.Light03_C"))
    (:`then_3`
      (`self.AddAbility` "Strong01" "/Game/Blueprints/Player/Abilities/Attacks/Strong01.Strong01_C"))
    (:`then_4`
      (`self.AddAbility` "Strong02" "/Game/Blueprints/Player/Abilities/Attacks/Strong02.Strong02_C"))
    (:`then_5`
      (`self.AddAbility` "Strong03" "/Game/Blueprints/Player/Abilities/Attacks/Strong03.Strong03_C"))
    (:`then_6`
      (`self.AddAbility` "Dodge" "/Game/Blueprints/Player/Abilities/Dodges/Dodge.Dodge_C"))))